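; Inventory Blueprint that holds a list of items, each with name, quantity and damage, capped at five entries.
; AddItemToInventory copies name-matched entries from ItemList, or prints a message when full.
; SubstractItem and AdditionItem find SelectedItem by name and adjust its quantity by one, but only when it is zero or less.
; Both print "Cannot find Item" after the loop even on a match; the other functions are empty stubs.
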(event Custom|AddItemToInventory
  (params (Name :type Text))
  (bind _inventory (Variables|Default|GetInventory))
  ;[0.15 0.15 0.15 0.5] Add the selected item to the inventory (if inventory size is 5 or more, refuse and show message)
  (if (< (Utilities|Array|Length _inventory) 5)
    (for _array_element (Variables|Default|GetItemList)
      (if (Utilities|Enum|Equal(Enum) (.name _array_element) Name)
        (Utilities|Array|Add _inventory (Utilities|Struct|MakeS_StructItem (.name _array_element) (.quantity _array_element) (.damage _array_element)))))
    (else
      (Development|PrintText "Inventory full"))))

(event Custom|SubstractItem
  (bind _inventory (Variables|Default|GetInventory))
  ;[0.15 0.15 0.15 0.5] Find the item in the inventory and subtract the item by 1
  (for (_array_element _array_index) _inventory
    (if (Utilities|Enum|Equal(Enum) (.name (Variables|Default|GetSelectedItem)) (.name _array_element))
      (if (<= (.Quantity (Utilities|Struct|BreakS_StructItem (Utilities|Array|Get(acopy) _inventory _array_index))) 0)
        (Utilities|Array|SetArrayElem _inventory _array_index (Utilities|Struct|MakeS_StructItem (.Name (Utilities|Struct|BreakS_StructItem (Utilities|Array|Get(acopy) _inventory _array_index))) (- (.Quantity (Utilities|Struct|BreakS_StructItem (Utilities|Array|Get(acopy) _inventory _array_index))) 1) (.Damage (Utilities|Struct|BreakS_StructItem (Utilities|Array|Get(acopy) _inventory _array_index)))))
        (else
          (Development|PrintText "Item cannot be subtracted")))))
  (Development|PrintText "Cannot find Item"))

(event Custom|AdditionItem
  (bind _inventory (Variables|Default|GetInventory))
  ;[0.15 0.15 0.15 0.5] Find the item in the inventory and subtract the item by 1
  (for (_array_element _array_index) _inventory
    (if (Utilities|Enum|Equal(Enum) (.name (Variables|Default|GetSelectedItem)) (.name _array_element))
      (if (<= (.Quantity (Utilities|Struct|BreakS_StructItem (Utilities|Array|Get(acopy) _inventory _array_index))) 0)
        (Utilities|Array|SetArrayElem _inventory _array_index (Utilities|Struct|MakeS_StructItem (.Name (Utilities|Struct|BreakS_StructItem (Utilities|Array|Get(acopy) _inventory _array_index))) (+ (.Quantity (Utilities|Struct|BreakS_StructItem (Utilities|Array|Get(acopy) _inventory _array_index))) 1) (.Damage (Utilities|Struct|BreakS_StructItem (Utilities|Array|Get(acopy) _inventory _array_index)))))
        (else
          (Development|PrintText "Item cannot be subtracted")))))
  (Development|PrintText "Cannot find Item"))

(event EventBeginPlay)

(event EventTick
  (params (DeltaSeconds :type Float%20%28single-precision%29)))

(fn NewFunction
  (return))

(fn NewFunction0)