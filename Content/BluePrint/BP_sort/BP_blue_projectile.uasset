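; BP_blue_projectile is a projectile that flies toward an optional Target and is destroyed on hit.
; The construction script applies Speed and Gravity to ProjectileMovement and enables homing on the Target's root component when Ishomming is set.
; On BeginPlay, a valid Target sets the initial velocity toward it.
; Box collision hits trigger CallImpact before destruction; the node to ignore the owner during movement is unconnected.
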(event OnComponentHit(Boxcolision)
  (params (HitComponent :type Primitive%20Component%20Object%20Reference) (OtherActor :type Actor%20Object%20Reference) (OtherComp :type Primitive%20Component%20Object%20Reference) (NormalImpulse :type Vector :default "0, 0, 0") (Hit :type Hit%20Result%20Structure%20%28by%20ref%29))
  (Default|CallImpact OtherActor Hit)
  (Actor|DestroyActor))

(event Custom|Rotate%20to%20target
  (Variables|/Script/Engine.MovementComponent|SetVelocity (Variables|Default|GetProjectileMovement) (* (Math|Vector|GetUnitDirection(Vector) (Transformation|GetActorLocation) (Transformation|GetActorLocation (Variables|target|GetTarget))) (Variables|prjectilesettings|Getspeed))))

(event EventBeginPlay
  (Variables|target|GetTarget
    (:then
      (CallFunction|RotatetoTarget))
    (:else)))

(fn ConstructionScript
  (bind _projectilemovement (Variables|Default|GetProjectileMovement))
  (Variables|/Script/Engine.ProjectileMovementComponent|SetInitialSpeed _projectilemovement (Variables|prjectilesettings|Getspeed))
  (Variables|/Script/Engine.ProjectileMovementComponent|SetMaxSpeed _projectilemovement (Variables|prjectilesettings|Getspeed))
  (Variables|/Script/Engine.ProjectileMovementComponent|SetProjectileGravityScale _projectilemovement (Variables|prjectilesettings|Getgravity))
  (Variables|target|GetTarget
    (:then
      (if (Variables|prjectilesettings|GetIshomming)
        (Variables|/Script/Engine.ProjectileMovementComponent|SetbIsHomingProjectile _projectilemovement true)
        (Variables|/Script/Engine.ProjectileMovementComponent|SetHomingTargetComponent _projectilemovement (Variables|/Script/Engine.Actor|GetRootComponent (Variables|target|GetTarget)))))
    (:else)))