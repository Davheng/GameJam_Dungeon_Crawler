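; Turn battle controller that sketches a player-versus-enemy combat flow using debug prints, with no attack logic yet.
; On BeginPlay, InitCombat resets the turn count and battle state, then starts PlayerTurn.
; PlayerTurn prints a win if Ennemie is dead, otherwise hands off to EnnemieTurn.
; EnnemieTurn stops after casting the player character, as its HP game-over check and loop back to PlayerTurn are unconnected.
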(event EventBeginPlay
  (CallFunction|InitCombat))

(event Collision|EventActorBeginOverlap
  (params (OtherActor :type Actor%20Object%20Reference)))

(event EventTick
  (params (DeltaSeconds :type Float%20%28single-precision%29)))

(fn ConstructionScript)

(fn InitCombat
  (Variables|Default|SetTurnCount 0)
  (Variables|Default|SetBattleState 0)
  (CallFunction|PlayerTurn))

(fn PlayerTurn
  (Development|PrintText "Player Turn")
  (bind _newparam (Default|IsAlive (Variables|Default|Getennemie)))
  (if _newparam
    (CallFunction|EnnemieTurn)
    (else
      (Development|PrintText "yay i win"))))

(fn EnnemieTurn
  (Development|PrintString "EnnemieTurn")
  (bind _asbp_first_person_character (Utilities|Casting|CastToBP_FirstPersonCharacter (Game|GetPlayerCharacter 0))))