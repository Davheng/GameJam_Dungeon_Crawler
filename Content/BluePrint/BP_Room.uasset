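; Room segment that procedurally extends the level along +X when the player enters it.
; When BP_FirstPersonCharacter overlaps its Box, it spawns two BP_Corridor actors and another BP_Room, each offset in X from the previous spawn point, starting at the Box location.
; Each new room carries the same trigger, so the chain can continue indefinitely.
; Nothing guards against repeat overlaps or removes earlier segments.
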(event OnComponentBeginOverlap(Box)
  (params (OverlappedComponent :type Primitive%20Component%20Object%20Reference) (OtherActor :type Actor%20Object%20Reference) (OtherComp :type Primitive%20Component%20Object%20Reference) (OtherBodyIndex :type Integer) (bFromSweep :type Boolean) (SweepResult :type Hit%20Result%20Structure%20%28by%20ref%29))
  (bind _returnvalue (Transformation|GetWorldLocation OverlappedComponent))
  (bind (_x _y _z) (Math|Vector|BreakVector _returnvalue))
  (bind _returnvalue_2 (+ _x 2e+03))
  (bind _returnvalue_3 (Math|Vector|MakeVector _returnvalue_2 _y _z))
  (bind (_x_2 _y_2 _z_2) (Math|Vector|BreakVector _returnvalue_3))
  (bind _returnvalue_4 (+ _x_2 2.5e+03))
  (bind _returnvalue_5 (Math|Vector|MakeVector _returnvalue_4 _y_2 _z_2))
  (bind (_x_3 _y_3 _z_3) (Math|Vector|BreakVector _returnvalue_5))
  (Utilities|Casting|CastToBP_FirstPersonCharacter OtherActor)
  (Game|SpawnActorfromClass "/Game/BluePrint/BP_Corridor.BP_Corridor_C" (Math|Transform|MakeTransform _returnvalue_3 "0, 0, 0" "1.000000,1.000000,1.000000") "Undefined" "MultiplyWithRoot" 0 0)
  (Game|SpawnActorfromClass "/Game/BluePrint/BP_Corridor.BP_Corridor_C" (Math|Transform|MakeTransform _returnvalue_5 "0, 0, 0" "1.000000,1.000000,1.000000") "Undefined" "MultiplyWithRoot" 0 0)
  (Game|SpawnActorfromClass "BP_Room_C" (Math|Transform|MakeTransform (Math|Vector|MakeVector (+ _x_3 2.5e+03) _y_3 _z_3) "0, 0, 0" "1.000000,1.000000,1.000000") "Undefined" "MultiplyWithRoot" 0 0))

(event EventBeginPlay)

(event Collision|EventActorBeginOverlap
  (params (OtherActor :type Actor%20Object%20Reference)))

(event EventTick
  (params (DeltaSeconds :type Float%20%28single-precision%29)))

(fn ConstructionScript)