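; BattleSys runs an automatic turn-based fight between the first-person player and an enemy passed into InitFight.
; PlayerTurn damages the enemy with inventory items, cycled by turn count, and does nothing if the inventory is empty.
; EnemyTurn applies enemy damage via ChangeHP, then calls PlayerTurn again without delay or input until one side dies.
; A win restores walking movement, while a loss prints game over.
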(event Custom|InitFight
  (params (Enemy :type Ennemies%20Object%20Reference))
  (Variables|Default|SetEnemy Enemy)
  (CallFunction|PlayerTurn))

(event Custom|PlayerTurn
  (bind _enemy (Variables|Default|GetEnemy))
  (bind _firstpersonchar (Variables|Default|GetFirstPersonChar))
  (bind _enemycomp (Variables|/Game/BluePrint/Ennemies/Ennemies.Ennemies_C|GetEnemyComp _enemy))
  (bind _inventorysystem (Variables|/Game/FirstPerson/Blueprints/BP_FirstPersonCharacter.BP_FirstPersonCharacter_C|GetInventorySystem _firstpersonchar))
  (bind _inventory (Variables|/Game/Items/Blueprint/Inventory.Inventory_C|GetInventory _inventorysystem))
  (bind _returnvalue (Utilities|Array|Length _inventory))
  ;[0.15 0.15 0.15 0.5] Player
  (if (not (<= _returnvalue 0))
    (Development|PrintText "Player Turn")
    (Default|GetDamage _enemycomp (.Damage (Utilities|Struct|BreakS_StructItem (Utilities|Array|Get(acopy) _inventory (Math|Integer|%(Integer) (Variables|Default|GetTurns) _returnvalue)))))
    (bind _status (Default|IsAlive _enemycomp))
    (if _status
      (CallFunction|EnemyTurn)
      (else
        (Pawn|Components|CharacterMovement|SetMovementMode (Variables|/Script/Engine.Character|GetCharacterMovement (Variables|Default|GetFirstPersonChar)) "MOVE_Walking" 0)))))

(event Custom|EnemyTurn
  (bind _firstpersonchar (Variables|Default|GetFirstPersonChar))
  ;[0.15 0.15 0.15 0.5] Enemy
  (Development|PrintString "EnnemieTurn")
  (Default|ChangeHP _firstpersonchar (.damage (Variables|/Game/BluePrint/Ennemies/EnemyComp.EnemyComp_C|GetStats (Variables|/Game/BluePrint/Ennemies/Ennemies.Ennemies_C|GetEnemyComp (Variables|Default|GetEnemy)))))
  (bind _newparam (Default|IsAlive _firstpersonchar))
  (if _newparam
    (bind _output_get (Variables|Default|SetTurns (+ (Variables|Default|GetTurns) 1)))
    (Development|PrintText (Utilities|Text|ToText(Integer) _output_get))
    (CallFunction|PlayerTurn)
    (else
      (Development|PrintText "game over"))))

(event EventBeginPlay
  (bind _asbp_first_person_character (Utilities|Casting|CastToBP_FirstPersonCharacter (Game|GetPlayerCharacter 0)))
  (Variables|Default|SetFirstPersonChar _asbp_first_person_character))

(event EventTick
  (params (DeltaSeconds :type Float%20%28single-precision%29)))